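; BP_HealthComponent is a health component that tracks current health against a maximum.
; On BeginPlay it sets CurrentHealth to MaxHealth.
; ReceiveDamage subtracts the incoming damage without clamping and prints the new value.
; Its check for health at or below zero has no logic attached, so death is not handled here.
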(event `self.ReceiveBeginPlay`
  (set `self.CurrentHealth` (`self.MaxHealth`)))

(fn `ReceiveDamage`
  (params (Damage :type Integer))
  (bind _output_get (set `self.CurrentHealth` (- (`self.CurrentHealth`) Damage)))
  (`KismetSystemLibrary.PrintString` (`KismetStringLibrary.Conv_IntToString` (`self.CurrentHealth`)))
  (if (<= _output_get 0)
    _))