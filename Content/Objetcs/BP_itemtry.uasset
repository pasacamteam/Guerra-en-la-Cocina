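; BP_itemtry is an item Blueprint that boosts the player character's speed when its item action runs.
; It overrides ItemAction, calls the parent version, then casts player pawn 0 to BP_TopDownCharacter and passes its current speed plus a fixed bonus to SpeedChange.
; The graph contains no timer or reset for the boost, and its other events only hold disabled or parent-call stubs.
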(fn `ItemAction`
  (`parent.ItemAction`)
  (bind _asbp_top_down_character (cast `/Game/TopDown/Blueprints/BP_TopDownCharacter` (`GameplayStatics.GetPlayerPawn` 0)))
  (bind _maxwalkspeed (`/Game/TopDown/Blueprints/BP_TopDownCharacter.GetSpeed` _asbp_top_down_character))
  (`/Game/TopDown/Blueprints/BP_TopDownCharacter.SpeedChange` _asbp_top_down_character (+ _maxwalkspeed 1000.0)))

(fn `UserConstructionScript`
  (`parent.UserConstructionScript`))