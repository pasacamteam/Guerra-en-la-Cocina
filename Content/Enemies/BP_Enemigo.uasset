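; BP_Enemigo is an enemy that chases the player using a looping AI MoveTo, re-issued one second after each successful move.
; Its health component triggers a placeholder Niagara hit effect on damage.
; On death it notifies the RoundManager of the elimination and destroys itself.
; Static mesh hits set a brief InHitstun flag, which gates only repeat hits here and does not interrupt the chase.
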(event `Damage Effect`
  (`NiagaraFunctionLibrary.SpawnSystemAtLocation` "/Game/Particles/NS_HitPlaceholder.NS_HitPlaceholder" (`self.K2_GetActorLocation`)))

(event `self.ReceiveBeginPlay`
  (`|ExecutionSequence`
    (:`then_0`
      (add `/Game/Components/BP_HealthComponent.OnDamageReceived` (`self.BP_HealthComponent`) (delegate `Damage Effect`)))
    (:`then_1`
      (`self.Perseguir`))))

(event `Perseguir`
  (`|AIMoveTo` self (0.0 0.0 0.0) (`GameplayStatics.GetPlayerCharacter` 0)
    (:`OnSuccess`
      (`KismetSystemLibrary.Delay` 1.0)
      (`self.Perseguir`))))

(event `self.CapsuleComponent.OnComponentBeginOverlap`
  (params (OverlappedComponent :type "PrimitiveComponent Object Reference") (OtherActor :type "Actor Object Reference") (OtherComp :type "PrimitiveComponent Object Reference") (OtherBodyIndex :type Integer) (bFromSweep :type Boolean) (SweepResult :type "HitResult Structure (by ref)")))

(event `self.StaticMesh.OnComponentHit`
  (params (HitComponent :type "PrimitiveComponent Object Reference") (OtherActor :type "Actor Object Reference") (OtherComp :type "PrimitiveComponent Object Reference") (NormalImpulse :type "Vector Structure") (Hit :type "HitResult Structure (by ref)"))
  (if (not (`self.In Hitstun`))
    (set `self.In Hitstun` true)
    (`KismetSystemLibrary.Delay` 0.5)
    (set `self.In Hitstun` false)))

(event `self.BP_HealthComponent.AlMorir`
  (`KismetSystemLibrary.PrintString` "Im dead :(")
  (bind _returnvalue (`GameplayStatics.GetActorOfClass` "/Game/TopDown/Blueprints/RoundManager.RoundManager_C"))
  (`/Game/TopDown/Blueprints/RoundManager.EliminateEnemyRM` _returnvalue)
  (`self.K2_DestroyActor`))

(fn `UserConstructionScript`)